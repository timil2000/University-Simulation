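; Blueprint function library for the quiz game that gates feedback and text on the player's settings stored in BP_GameInstance.
; PlaySound plays a 2D sound and PlayVibration spawns the FFE_Fire force feedback, each only when its setting is enabled.
; TranslateLanguage picks between English and Other strings passed by the caller, based on the selected language.
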(fn `PlaySound`
  (params (Sound :type "SoundBase Object Reference"))
  (bind _asbp_game_instance (cast `/Game/Quiz_Game/Blueprints/BP_GameInstance` (`GameplayStatics.GetGameInstance` null)))
  (if (`/Game/Quiz_Game/Blueprints/BP_GameInstance.EnabledSounds` _asbp_game_instance)
    (`GameplayStatics.PlaySound2D` null Sound 1.0 1.0 0.0 null null))
  (return))

(fn `PlayVibration`
  (bind _asbp_game_instance (cast `/Game/Quiz_Game/Blueprints/BP_GameInstance` (`GameplayStatics.GetGameInstance` null)))
  (if (`/Game/Quiz_Game/Blueprints/BP_GameInstance.EnabledVibration` _asbp_game_instance)
    (`GameplayStatics.SpawnForceFeedbackAtLocation` null "/Game/Quiz_Game/Blueprints/FFE_Fire.FFE_Fire" (0.0 0.0 0.0) (struct) false 1.0 0.0 null))
  (return))

(fn `TranslateLanguage`
  (params (English :type Text) (Other :type Text))
  (returns (ReturnValue :type Text))
  (bind _asbp_game_instance (cast `/Game/Quiz_Game/Blueprints/BP_GameInstance` (`GameplayStatics.GetGameInstance` null)))
  (return (select `/Game/Quiz_Game/Blueprints/E_Languages` (`/Game/Quiz_Game/Blueprints/BP_GameInstance.Selected_Language` _asbp_game_instance) :`NewEnumerator0` English :`NewEnumerator1` Other)))